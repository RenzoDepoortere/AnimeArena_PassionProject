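; Base character Blueprint that drives an on-screen debug readout of its speed level and current state.
; On BeginPlay it creates a WB_Debug widget for the first player controller, adds it to the viewport and binds to the speed switch dispatcher.
; Speed switch events and the StateMachineComponent's state switch events push their values into the widget's text, so no Tick polling is used.
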(event `self.ReceiveBeginPlay`
  (bind _returnvalue (`|CreateWidget` "/Game/Blueprints/UI/WB_Debug.WB_Debug_C" (`GameplayStatics.GetPlayerController` 0)))
  (bind _output_get (set `self.DebugWidget` _returnvalue))
  (`UserWidget.AddToViewport` _output_get 0)
  (add `self.OnSpeedSwitch` (delegate `SpeedSwitch`)))

(event `SpeedSwitch` :!signature `self.OnSpeedSwitch`
  (params (speedLevel :type Integer))
  (set `/Game/Blueprints/UI/WB_Debug.LevelText` (`KismetStringLibrary.Conv_IntToString` speedLevel) (`self.DebugWidget`)))

(event `self.ReceiveTick`
  (params (DeltaSeconds :type "Float (single-precision)")))

(event `self.StateMachineComponent.OnStateSwitch`
  (params (stateKey :type String))
  (set `/Game/Blueprints/UI/WB_Debug.StateText` stateKey (`self.DebugWidget`)))

(fn `UserConstructionScript`)